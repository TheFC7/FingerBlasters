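; Gameplay player controller that spawns the player's chosen character and runs multiplayer text chat.
; On BeginPlay the local controller loads saved player info and passes it toward the server, where the GameplayGM game mode respawns the character before the chat widget is created.
; Chat messages are tagged with the player's name and relayed through every controller in the game mode's list to update each chat window.
; The T key toggles the mouse cursor for typing.
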(event Custom|PassCharacterInfoToServer
  (params (PlayerSettingsInfo :type Player%20Info%20Structure))
  ;[1 1 1] Passes character info / respawns player with selected character / calls chat window
  (Variables|Default|SetPlayerSettings PlayerSettingsInfo)
  (bind _asgameplay_gm (Utilities|Casting|CastToGameplayGM (Game|GetGameMode)))
  (Default|RespawnPlayer _asgameplay_gm self (.MyPlayerCharacter (Utilities|Struct|BreakPlayerInfo (Variables|Default|GetPlayerSettings))))
  (CallFunction|SetupChatWindow))

(event Custom|SetupChatWindow
  ;[1 1 1] Creates gameplay chat and viewport
  (bind _returnvalue (UserInterface|CreateWidget "/Game/UI/AllLevels/GameplayChat.GameplayChat_C"))
  (bind _output_get (Variables|Default|SetGameplayChatWB _returnvalue))
  (UserInterface|Viewport|AddtoViewport _output_get 0))

(event Custom|GetChatMessage
  (params (TextToSend :type Text))
  ;[1 1 1] Process and handles chat, calls and updates chat on client
  (Variables|Default|SetSenderText TextToSend)
  (Variables|Default|SetSenderName (.MyPlayerName (Utilities|Struct|BreakPlayerInfo (Variables|Default|GetPlayerSettings))))
  (bind _asgameplay_gm (Utilities|Casting|CastToGameplayGM (Game|GetGameMode)))
  (for _array_element (Variables|/Game/Blueprints/Gamemode/GameplayGM.GameplayGM_C|GetAllPlayerControllers _asgameplay_gm)
    (bind _asgameplay_pc (Utilities|Casting|CastToGameplayPC _array_element))
    (CallFunction|UpdateChat _asgameplay_pc (Variables|Default|GetSenderName) (Variables|Default|GetSenderText))))

(event Custom|UpdateChat
  (params (SenderName :type Text) (SenderText :type Text))
  ;[1 1 1] Updates clientside chat window
  (Default|UpdateChatWindow (Variables|/Game/UI/AllLevels/GameplayChat.GameplayChat_C|GetGameplayChat (Variables|Default|GetGameplayChatWB)) SenderName SenderText))

(event EventBeginPlay
  ;[1 1 1] Loads Player info, pass to server side player controller
  (if (Pawn|IsLocalController)
    (Viewport|RemoveAllWidgets)
    (CallFunction|LoadGame)
    (CallFunction|PassCharacterInfotoServer (Variables|Default|GetPlayerSettings))))

(event Input|KeyboardEvents|T
  (params (Key :type Key%20Structure))
  ;[1 1 1] T to type
  (:Pressed
    (Utilities|FlowControl|FlipFlop
      (:A
        (Variables|Default|SetbShowMouseCursor true))
      (:B
        (Variables|Default|SetbShowMouseCursor false)))))

(fn ConstructionScript)

(fn LoadGame
  (bind _returnvalue (SaveGame|LoadGamefromSlot (Variables|Default|GetPlayerSettingsSave)))
  (bind _asplayer_save_game (Utilities|Casting|CastToPlayerSaveGame _returnvalue))
  (Variables|Default|SetPlayerSettings (Variables|/Game/Blueprints/AllLevels/Playersavegame.PlayerSaveGame_C|GetS_PlayerInfo _asplayer_save_game)))